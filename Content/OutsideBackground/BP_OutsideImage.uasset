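; BP_OutsideImage is an outside-background actor that keeps turning to face the player, like a yaw-only billboard.
; BeginPlay caches the player character as a BP_Character reference.
; Each Tick finds the look-at rotation toward that character, interpolates toward it with RInterpTo and applies only the yaw, so the actor stays upright.
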(event `self.ReceiveBeginPlay`
  (bind _asbp_character (cast `/Game/_HorrorGame/Core/Characters/BP_Character` (`GameplayStatics.GetPlayerCharacter` 0)))
  (set `self.PlayerReference` _asbp_character))

(event `self.ReceiveTick`
  (params (DeltaSeconds :type "Float (single-precision)"))
  (bind (_returnvalue_roll _returnvalue_pitch _returnvalue_yaw) (`KismetMathLibrary.BreakRotator` (`self.K2_GetActorRotation`)))
  (bind (_returnvalue_roll_2 _returnvalue_pitch_2 _returnvalue_yaw_2) (`KismetMathLibrary.BreakRotator` (`KismetMathLibrary.RInterpTo` (`KismetMathLibrary.MakeRotator` 0.0 0.0 _returnvalue_yaw) (`KismetMathLibrary.FindLookAtRotation` (`self.K2_GetActorLocation`) (`self.K2_GetActorLocation` (`self.PlayerReference`))) (`GameplayStatics.GetWorldDeltaSeconds`) 20.0)))
  (`self.K2_SetActorRotation` (`KismetMathLibrary.MakeRotator` 0.0 0.0 _returnvalue_yaw_2)))

(fn `UserConstructionScript`)