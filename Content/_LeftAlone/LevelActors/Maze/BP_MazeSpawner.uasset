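; BP_MazeSpawner starts the maze sequence once a specific dialogue finishes.
; On the tick after BeginPlay it binds to the game mode's ACTC dialogue manager, and a matching dialogue key fires the start once via DoOnce.
; Starting the maze spawns a witch enemy just above the first BP_SpawnPoint found, moves the player to the spawner's own location and plays the maze sound.
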(event `self.ReceiveBeginPlay`
  (`KismetSystemLibrary.DelayUntilNextTick`)
  (bind _asbp_game_mode (cast `/Game/_LeftAlone/Core/GameModes/Gameplay/BP_GameMode` (`GameplayStatics.GetGameMode`)))
  (add `/Game/_LeftAlone/Core/DialogueSystem/ACTC_DialogueManager.OnCompleteDialogue` (`/Game/_LeftAlone/Core/GameModes/Gameplay/BP_GameMode.ACTC_DialogueManager` _asbp_game_mode) (delegate `OnCompleteDialogue_Event`)))

(event `OnCompleteDialogue_Event`
  (params (`Dialogue Key` :type String))
  (if (`KismetStringLibrary.EqualEqual_StrStr` `Dialogue Key` (`self.DialogueEventToStartMaze`))
    (`/Engine/EditorBlueprintResources/StandardMacros.DoOnce` false
      (:`Completed`
        (`self.StartMaze`)))))

(event `StartMaze`
  (bind _outactors (`GameplayStatics.GetAllActorsOfClass` "/Game/_LeftAlone/Core/AISystem/AI/BP_SpawnPoint.BP_SpawnPoint_C"))
  (bind (_returnvalue_x _returnvalue_y _returnvalue_z) (`KismetMathLibrary.BreakVector` (`self.K2_GetActorLocation` (`|GetArrayItem` _outactors))))
  (`|SpawnActorFromClass` "/Game/_LeftAlone/Core/AISystem/AI/BP_Enemy_Witch.BP_Enemy_Witch_C" (`KismetMathLibrary.MakeTransform` (`KismetMathLibrary.MakeVector` _returnvalue_x _returnvalue_y (+ _returnvalue_z 150.0))) "AlwaysSpawn" "MultiplyWithRoot" null null)
  (bind _asbp_character (cast `/Game/_LeftAlone/Core/Characters/BP_Character` (`GameplayStatics.GetPlayerPawn` 0)))
  (`self.K2_SetActorLocation` _asbp_character (`self.K2_GetActorLocation`) false false)
  (`GameplayStatics.SpawnSound2D` "/Game/Music/ThiSound_Maze.ThiSound_Maze" 1.0 1.0 0.0 null))

(fn `UserConstructionScript`)