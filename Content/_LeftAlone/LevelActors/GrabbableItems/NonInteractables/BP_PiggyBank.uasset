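; BP_PiggyBank is a piggy bank prop that the player can pick up and release.
; On Interact it passes its physics handle, the player character's camera and the pig mesh to the ACTCGrab component, then calls that component's InteractMessage.
; InteractRelease releases the grabbed component directly through the physics handle.
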(event `/Game/_LeftAlone/Core/Interfaces/BPI_Interactable.Interact`
  (bind _asbp_character (cast `/Game/_LeftAlone/Core/Characters/BP_Character` (`GameplayStatics.GetPlayerCharacter` 0)))
  (bind _playercamera (`/Game/_LeftAlone/Core/Characters/BP_Character.PlayerCamera` _asbp_character)
    (:`then`
      (`/Game/_LeftAlone/Core/ActorComponents/ACTC_Grab.SetupGrabber` (`self.ACTC_Grab`) (`self.PhysicsHandlePiggy`) _playercamera (`self.StaticMeshPig`))
      (message `/Game/_LeftAlone/Core/Interfaces/BPI_Interactable.Interact` (`self.ACTC_Grab`)))
    (:`else`)))

(event `/Game/_LeftAlone/Core/Interfaces/BPI_Interactable.InteractRelease`
  (`PhysicsHandleComponent.ReleaseComponent` (`self.PhysicsHandlePiggy`)))

(fn `UserConstructionScript`)