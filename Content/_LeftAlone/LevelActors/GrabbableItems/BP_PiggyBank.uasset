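; BP_PiggyBank is a grabbable piggy bank level item that can be picked up and released through physics.
; BeginPlay caches the player BP_Character and, if valid, its camera.
; Grab attaches the static mesh to a PhysicsHandle at the actor's location and rotation and enables ticking on the ACTCGrab component.
; Release drops the mesh and disables that tick, so the component only ticks while held.
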(event `self.ReceiveBeginPlay`
  (bind _asbp_character (cast `/Game/_LeftAlone/Core/Characters/BP_Character` (`GameplayStatics.GetPlayerCharacter` 0)))
  (bind _output_get (set `self.CharacterReference` _asbp_character))
  (bind _playercamera (`/Game/_LeftAlone/Core/Characters/BP_Character.PlayerCamera` _output_get)
    (:`then`
      (set `self.CharacterCameraReference` _playercamera))
    (:`else`)))

(event `/Game/_LeftAlone/Core/Interfaces/BPI_Grabbable.Grab`
  (`PhysicsHandleComponent.GrabComponentAtLocationWithRotation` (`self.PhysicsHandle`) (`self.StaticMesh`) "None" (`self.K2_GetActorLocation`) (`self.K2_GetActorRotation`))
  (`ActorComponent.SetComponentTickEnabled` (`self.ACTC_Grab`) true))

(event `/Game/_LeftAlone/Core/Interfaces/BPI_Grabbable.Release`
  (`PhysicsHandleComponent.ReleaseComponent` (`self.PhysicsHandle`))
  (`ActorComponent.SetComponentTickEnabled` (`self.ACTC_Grab`) false))

(fn `UserConstructionScript`)