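; BP_DoorGrabbable is a door actor the player can grab and swing by moving the mouse horizontally.
; Grab enables input on the actor and locks camera look; Release reverses both.
; While grabbed, scaled mouse input adds yaw to the Door component without angle limits, with a dot product flipping direction by the player's side.
; Debug prints remain in Grab and Tick, and OnObjectGrab is an empty stub.
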(event `self.ReceiveBeginPlay`
  (bind _asbp_character (cast `/Game/_LeftAlone/Core/Characters/BP_Character` (`GameplayStatics.GetPlayerCharacter` 0)))
  (set `self.As BP Character` _asbp_character))

(event `/Game/_LeftAlone/Core/Interfaces/BPI_NewGrabbable.Grab`
  (bind _returnvalue (`GameplayStatics.GetPlayerController` 0))
  (`Controller.SetIgnoreLookInput` _returnvalue true)
  (`self.EnableInput` _returnvalue)
  (`KismetSystemLibrary.PrintString` "Hello"))

(event `/Game/_LeftAlone/Core/Interfaces/BPI_NewGrabbable.Release`
  (bind _returnvalue (`GameplayStatics.GetPlayerController` 0))
  (`Controller.ResetIgnoreLookInput` _returnvalue)
  (`self.DisableInput` _returnvalue))

(event `InputAxis|HorizontalMouse`
  (params (AxisValue :type "Float (single-precision)"))
  (bind _door (`self.Door`))
  (`SceneComponent.K2_SetRelativeRotation` _door (`KismetMathLibrary.ComposeRotators` (`SceneComponent.RelativeRotation` _door) (`KismetMathLibrary.MakeRotator` 0.0 0.0 (* (* AxisValue 0.8) (select `bool` (>= (`KismetMathLibrary.Dot_VectorVector` (`KismetMathLibrary.Normal` (- (`self.K2_GetActorLocation`) (`self.K2_GetActorLocation` (`self.As BP Character`)))) (`self.GetActorForwardVector`)) 0.0) :`false` 1.0 :`true` -1.0)))) false false))

(event `self.ReceiveTick`
  (params (DeltaSeconds :type "Float (single-precision)"))
  ;[1 1 1] debug dot product
  (`KismetSystemLibrary.PrintText` (`KismetTextLibrary.Conv_DoubleToText` 0.0 "HalfToEven") true true (struct :`G` 0.66 :`B` 1.0 :`A` 1.0) DeltaSeconds))

(fn `OnObjectGrab`
  (returns (GrabbedItem :type "PrimitiveComponent Object Reference")))

(fn `UserConstructionScript`)