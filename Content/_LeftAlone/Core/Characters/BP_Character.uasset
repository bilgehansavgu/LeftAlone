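; First-person player character that handles gated look and movement input, adds a crosshair, and lets the player interact, grab objects and advance dialogue.
; A short camera line trace finds interface-implementing actors to interact with or hold through a PhysicsHandle.
; Space advances the game mode's dialogue manager, and F starts the maze spawner.
; RotateToActor disables controller-driven rotation and uses a timeline to turn view and body toward a target.
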(event `self.ReceiveBeginPlay`
  (bind _actc_grab (`self.ACTC_Grab`))
  (bind _returnvalue (`|CreateWidget` "/Game/_LeftAlone/Widgets/Crosshair/WBP_Crosshair.WBP_Crosshair_C"))
  ;[1 1 1] hmmm
  (`UserWidget.AddToViewport` _returnvalue 0)
  (`ActorComponent.Deactivate` _actc_grab)
  (`ActorComponent.SetComponentTickEnabled` _actc_grab false)
  (bind _asbp_game_mode (cast `/Game/_LeftAlone/Core/GameModes/Gameplay/BP_GameMode` (`GameplayStatics.GetGameMode`)))
  (set `self.Ref BP Game Mode` _asbp_game_mode))

(event `InputAxis|VerticalMouse`
  (params (AxisValue :type "Float (single-precision)"))
  ;[1 1 1] Movement
  (if (`self.canMove`)
    (`self.AddControllerPitchInput` AxisValue)))

(event `InputAxis|HorizontalMouse`
  (params (AxisValue :type "Float (single-precision)"))
  ;[1 1 1] Movement
  (if (`self.canMove`)
    (`self.AddControllerYawInput` AxisValue)))

(event `InputAxis|VerticalMove`
  (params (AxisValue :type "Float (single-precision)"))
  ;[1 1 1] Movement
  (if (`self.canMove`)
    (`self.AddMovementInput` (`KismetMathLibrary.GetAxes` (`self.GetControlRotation`)) AxisValue)))

(event `InputAxis|HorizontalMove`
  (params (AxisValue :type "Float (single-precision)"))
  ;[1 1 1] Movement
  (if (`self.canMove`)
    (`self.AddMovementInput` (`.Y` (`KismetMathLibrary.GetAxes` (`self.GetControlRotation`))) AxisValue)))

(event `InputAction|InteractAction`
  (params (Key :type "Key Structure"))
  ;[1 1 1] Interaction
  (:`Pressed`
    (bind _hitactor (`self.LineTrace` 300.0))
    (if (and (`KismetSystemLibrary.IsValid` _hitactor) (`KismetSystemLibrary.DoesImplementInterface` _hitactor "/Game/_LeftAlone/Core/Interfaces/BPI_Interactable.BPI_Interactable_C"))
      (message `/Game/_LeftAlone/Core/Interfaces/BPI_Interactable.Interact` _hitactor))))

(event `InputAction|LeftClickAction`
  (params (Key :type "Key Structure"))
  (bind _physicshandle (`self.PhysicsHandle`))
  ;[1 1 1] Grab
  (:`Pressed`
    (bind (_hitactor _impactpoint) (`self.LineTrace` 300.0))
    (if (and (`KismetSystemLibrary.IsValid` _hitactor) (`KismetSystemLibrary.DoesImplementInterface` _hitactor "/Game/_LeftAlone/Core/Interfaces/BPI_Grabbable.BPI_Grabbable_C"))
      (bind _output_get (set `self.GrabbedObject` _hitactor))
      (bind _grabbeditem (message `/Game/_LeftAlone/Core/Interfaces/BPI_Grabbable.OnObjectGrab` _output_get))
      (`PhysicsHandleComponent.GrabComponentAtLocationWithRotation` _physicshandle _grabbeditem "None" _impactpoint (`SceneComponent.K2_GetComponentRotation` _grabbeditem))
      (message `/Game/_LeftAlone/Core/Interfaces/BPI_Grabbable.EnabledTick` _output_get true)
      (message `/Game/_LeftAlone/Core/Interfaces/BPI_Grabbable.SetupObject` _output_get _physicshandle (`self.Camera`))))
  (:`Released`
    (message `/Game/_LeftAlone/Core/Interfaces/BPI_Grabbable.OnObjectRelease` _output_get)
    (`PhysicsHandleComponent.ReleaseComponent` (`self.PhysicsHandle`))
    (message `/Game/_LeftAlone/Core/Interfaces/BPI_Grabbable.EnabledTick` _output_get false)))

(event `InputAction|SpaceAction`
  (params (Key :type "Key Structure"))
  ;[0.2969 0.00996 0.0455 1 20] todo:make sure player only can press space action when hes in dialogue for less buggyness
  (:`Pressed`
    (`/Game/_LeftAlone/Core/DialogueSystem/ACTC_DialogueManager.KeepTalking` (`/Game/_LeftAlone/Core/GameModes/Gameplay/BP_GameMode.ACTC_DialogueManager` (`self.Ref BP Game Mode`)))))

(event `RotateToActor`
  (params (Actor :type "Actor Object Reference"))
  (`/Engine/EditorBlueprintResources/StandardMacros.IsValid` Actor
    (:`Is Valid`
      (`self.EnableControls` false)
      (bind (_direction _rotationalpha) (`Timeline|FocusActorTimeline` :!via `PlayFromStart`)
        (:`Update`
          (bind _returnvalue (`KismetMathLibrary.RLerp` (`self.K2_GetActorRotation`) (`KismetMathLibrary.Conv_VectorToRotator` (`KismetMathLibrary.GetDirectionUnitVector` (`self.K2_GetActorLocation`) (`self.K2_GetActorLocation` Actor))) _rotationalpha true))
          (`SceneComponent.K2_SetWorldRotation` (`self.Camera`) _returnvalue false false)
          (`Controller.SetControlRotation` (`self.GetController`) _returnvalue)
          ;[1 1 1] check later if i need this, hmmm lol
          (`self.K2_SetActorRotation` _returnvalue))))
    (:`Is Not Valid`
      (`KismetSystemLibrary.PrintString` "bp_character rotate towards actor "))))

(event `Key|F`
  (params (Key :type "Key Structure"))
  (:`Pressed`
    (bind _returnvalue (`GameplayStatics.GetActorOfClass` "/Game/_LeftAlone/Core/Maze/BP_MazeSpawner.BP_MazeSpawner_C"))
    (`/Game/_LeftAlone/Core/Maze/BP_MazeSpawner.StartMaze` _returnvalue)))

(fn `EnableControls`
  (params (Controls :type Boolean))
  (set `CameraComponent.bUsePawnControlRotation` Controls (`self.Camera`))
  (set `self.bUseControllerRotationYaw` Controls))

(fn `LineTrace`
  (params (Distance :type "Float (double-precision)"))
  (returns (HitActor :type "Actor Object Reference") (ImpactPoint :type "Vector Structure"))
  (bind _camera (`self.Camera`))
  (bind _returnvalue (`SceneComponent.K2_GetComponentLocation` _camera))
  (bind _outhit (`KismetSystemLibrary.LineTraceSingle` :`Start` _returnvalue :`End` (+ _returnvalue (* Distance (`SceneComponent.GetForwardVector` _camera))) :`TraceChannel` "TraceTypeQuery1" :`DrawDebugType` "ForDuration"))
  (bind (_bblockinghit _binitialoverlap _time _distance _location _impactpoint _normal _impactnormal _physmat _hitactor) (`GameplayStatics.BreakHitResult` _outhit))
  (return _hitactor _impactpoint))

(fn `UserConstructionScript`)