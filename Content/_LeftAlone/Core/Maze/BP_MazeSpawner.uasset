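; BP_MazeSpawner is an actor that starts the maze sequence when a specific dialogue finishes.
; After a one-tick delay on BeginPlay, it binds to the dialogue manager held by BP_GameMode.
; When the completed key matches DialogueEventToStartMaze, a DoOnce-guarded StartMaze spawns BP_Enemy_Witch offset along world X and moves the player character to the spawner's location.
; StartMaze still carries a debug print.
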(event `self.ReceiveBeginPlay`
  (`KismetSystemLibrary.DelayUntilNextTick`)
  (bind _asbp_game_mode (cast `/Game/_LeftAlone/Core/GameModes/Gameplay/BP_GameMode` (`GameplayStatics.GetGameMode`)))
  (add `/Game/_LeftAlone/Core/DialogueSystem/ACTC_DialogueManager.OnCompleteDialogue` (`/Game/_LeftAlone/Core/GameModes/Gameplay/BP_GameMode.ACTC_DialogueManager` _asbp_game_mode) (delegate `OnCompleteDialogue_Event`)))

(event `OnCompleteDialogue_Event`
  (params (`Dialogue Key` :type String))
  (if (`KismetStringLibrary.EqualEqual_StrStr` `Dialogue Key` (`self.DialogueEventToStartMaze`))
    (`/Engine/EditorBlueprintResources/StandardMacros.DoOnce` false
      (:`Completed`
        (`self.StartMaze`)))))

(event `StartMaze`
  (bind (_returnvalue_x _returnvalue_y _returnvalue_z) (`KismetMathLibrary.BreakVector` (`self.K2_GetActorLocation`)))
  (`KismetSystemLibrary.PrintString` "f key")
  (`|SpawnActorFromClass` "/Game/_LeftAlone/Core/AISystem/AI/BP_Enemy_Witch.BP_Enemy_Witch_C" (`KismetMathLibrary.MakeTransform` (`KismetMathLibrary.MakeVector` (+ _returnvalue_x 1000.0) _returnvalue_y _returnvalue_z)) "Undefined" "MultiplyWithRoot" null null)
  (bind _asbp_character (cast `/Game/_LeftAlone/Core/Characters/BP_Character` (`GameplayStatics.GetPlayerPawn` 0)))
  (`self.K2_SetActorLocation` _asbp_character (`self.K2_GetActorLocation`) false false))

(fn `UserConstructionScript`)