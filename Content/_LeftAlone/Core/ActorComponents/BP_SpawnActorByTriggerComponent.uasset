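; Actor component that spawns an actor of a chosen class at its owner's transform when a selected dialogue completes.
; One tick after BeginPlay, it binds to the completion event of the dialogue manager on BP_GameMode.
; When the completed dialogue key matches the selected one, a DoOnce gate limits it to a single spawn.
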(event `self.ReceiveBeginPlay`
  (`KismetSystemLibrary.DelayUntilNextTick`)
  (bind _asbp_game_mode (cast `/Game/_LeftAlone/Core/GameModes/Gameplay/BP_GameMode` (`GameplayStatics.GetGameMode`)))
  (add `/Game/_LeftAlone/Core/DialogueSystem/ACTC_DialogueManager.OnCompleteDialogue` (`/Game/_LeftAlone/Core/GameModes/Gameplay/BP_GameMode.ACTC_DialogueManager` _asbp_game_mode) (delegate `OnCompleteDialogue_Event`)))

(event `OnCompleteDialogue_Event`
  (params (`Dialogue Key` :type String))
  (if (`KismetStringLibrary.EqualEqual_StrStr` `Dialogue Key` (`self.DialogSelectedToSpawn`))
    (`/Engine/EditorBlueprintResources/StandardMacros.DoOnce` false
      (:`Completed`
        (`|SpawnActorFromClass` (`self.ClassToSpawn`) (`Actor.GetTransform` (`self.GetOwner`)) "Undefined" "MultiplyWithRoot" null null)))))