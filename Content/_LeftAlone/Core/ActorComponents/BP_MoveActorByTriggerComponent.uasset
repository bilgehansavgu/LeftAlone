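; BP_MoveActorByTriggerComponent is an actor component that teleports its owner when a selected dialogue completes.
; One tick after BeginPlay, if a dialogue key is set, it binds to the game mode's dialogue manager completion event.
; A matching key moves the owner once, by a random offset from MoveLocations.
; A similar dialogue-play handler exists, but its Triggerer binding never runs.
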(event `self.ReceiveBeginPlay`
  (`KismetSystemLibrary.DelayUntilNextTick`)
  (if (not (`KismetStringLibrary.IsEmpty` (`self.DialogueSelectedToMove`)))
    (bind _asbp_game_mode (cast `/Game/_LeftAlone/Core/GameModes/Gameplay/BP_GameMode` (`GameplayStatics.GetGameMode`)))
    (bind _actc_dialoguemanager (`/Game/_LeftAlone/Core/GameModes/Gameplay/BP_GameMode.ACTC_DialogueManager` _asbp_game_mode)
      (:`then`
        (add `/Game/_LeftAlone/Core/DialogueSystem/ACTC_DialogueManager.OnCompleteDialogue` _actc_dialoguemanager (delegate `OnCompleteDialogue_Event`)))
      (:`else`))))

(event `OnCompleteDialogue_Event`
  (params (`Dialogue Key` :type String))
  (bind _returnvalue (`self.GetOwner`))
  (bind (_returnvalue_x _returnvalue_y _returnvalue_z) (`KismetMathLibrary.BreakVector` (+ (`Actor.K2_GetActorLocation` _returnvalue) (`KismetArrayLibrary.Array_Random` (`self.MoveLocations`)))))
  (if (`KismetStringLibrary.EqualEqual_StrStr` `Dialogue Key` (`self.DialogueSelectedToMove`))
    (`/Engine/EditorBlueprintResources/StandardMacros.DoOnce` false
      (:`Completed`
        (`Actor.K2_SetActorLocation` _returnvalue (`KismetMathLibrary.MakeVector` _returnvalue_x _returnvalue_y _returnvalue_z) false true)))))

(event `OnDialoguePlay_Event`
  (params (`Dialogue key` :type String) (`Actor to Focus` :type "Actor Object Reference"))
  (bind _returnvalue (`self.GetOwner`))
  (bind (_returnvalue_x _returnvalue_y _returnvalue_z) (`KismetMathLibrary.BreakVector` (+ (`Actor.K2_GetActorLocation` _returnvalue) (`KismetArrayLibrary.Array_Random` (`self.MoveLocations`)))))
  (`/Engine/EditorBlueprintResources/StandardMacros.DoOnce` false
    (:`Completed`
      (`Actor.K2_SetActorLocation` _returnvalue (`KismetMathLibrary.MakeVector` _returnvalue_x _returnvalue_y _returnvalue_z) false true))))