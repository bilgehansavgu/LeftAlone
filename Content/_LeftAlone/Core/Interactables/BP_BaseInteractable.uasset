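; BP_BaseInteractable is a base actor for interactable objects, storing a player character reference on BeginPlay.
; A highlight sphere overlap with BP_Character toggles highlighting through the ACTCHighligther component's message calls.
; The construction script hands the actor's StaticMesh to that component as the highlight target.
; The Interact event only prints a debug string.
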(event `self.ReceiveBeginPlay`
  (bind _asbp_character (cast `/Game/_LeftAlone/Core/Characters/BP_Character` (`GameplayStatics.GetPlayerCharacter` 0)))
  (set `self.PlayerReference` _asbp_character))

(event `/Game/_LeftAlone/Core/Interfaces/BPI_Interactable.Interact`
  (`KismetSystemLibrary.PrintString` "interact!"))

(event `self.SphereHighlight.OnComponentBeginOverlap`
  (params (OverlappedComponent :type "PrimitiveComponent Object Reference") (OtherActor :type "Actor Object Reference") (OtherComp :type "PrimitiveComponent Object Reference") (OtherBodyIndex :type Integer) (bFromSweep :type Boolean) (SweepResult :type "HitResult Structure (by ref)"))
  (cast `/Game/_LeftAlone/Core/Characters/BP_Character` OtherActor)
  (message `/Game/_LeftAlone/Core/Interfaces/BPI_HighlightActor.HighlightActor` (`self.ACTC_Highligther`) true))

(event `self.SphereHighlight.OnComponentEndOverlap`
  (params (OverlappedComponent :type "PrimitiveComponent Object Reference") (OtherActor :type "Actor Object Reference") (OtherComp :type "PrimitiveComponent Object Reference") (OtherBodyIndex :type Integer))
  (cast `/Game/_LeftAlone/Core/Characters/BP_Character` OtherActor)
  (message `/Game/_LeftAlone/Core/Interfaces/BPI_HighlightActor.HighlightActor` (`self.ACTC_Highligther`) false))

(fn `UserConstructionScript`
  ;[1 1 1] why did i make this an interface function i dont know
  (message `/Game/_LeftAlone/Core/Interfaces/BPI_HighlightActor.SetHighlightedActor` (`self.ACTC_Highligther`) (`self.StaticMesh`)))