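; Static Ouija board level actor for the horror game that highlights on overlap and configures a dialogue-keyed move component.
; On BeginPlay it registers its mesh with a highlighter component, and a Box overlap toggles that highlight on and off.
; It also passes its move locations and dialogue key to BPMoveActorByTriggerComponent.
; The branch that would assign a validated DialogueActor as that component's Triggerer is disconnected and never runs.
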(event `self.ReceiveBeginPlay`
  (bind _bp_moveactorbytriggercomponent (`self.BP_MoveActorByTriggerComponent`))
  (`|ExecutionSequence`
    (:`then_0`
      (`/Game/_HorrorGame/Core/ActorComponents/ACTC_Highligther.SetHighlightedActor` (`self.ACTC_Highligther`) (`self.StaticMeshComponent`)))
    (:`then_1`
      (set `/Game/_HorrorGame/Core/ActorComponents/BP_MoveActorByTriggerComponent.MoveLocations` (`self.MoveLocations`) _bp_moveactorbytriggercomponent)
      (set `/Game/_HorrorGame/Core/ActorComponents/BP_MoveActorByTriggerComponent.DialogueSelectedToMove` (`self.DialogueKey`) _bp_moveactorbytriggercomponent))))

(event `self.Box.OnComponentBeginOverlap`
  (params (OverlappedComponent :type "PrimitiveComponent Object Reference") (OtherActor :type "Actor Object Reference") (OtherComp :type "PrimitiveComponent Object Reference") (OtherBodyIndex :type Integer) (bFromSweep :type Boolean) (SweepResult :type "HitResult Structure (by ref)"))
  (`/Game/_HorrorGame/Core/ActorComponents/ACTC_Highligther.HighlightActor` (`self.ACTC_Highligther`) true))

(event `self.Box.OnComponentEndOverlap`
  (params (OverlappedComponent :type "PrimitiveComponent Object Reference") (OtherActor :type "Actor Object Reference") (OtherComp :type "PrimitiveComponent Object Reference") (OtherBodyIndex :type Integer))
  (`/Game/_HorrorGame/Core/ActorComponents/ACTC_Highligther.HighlightActor` (`self.ACTC_Highligther`) false))

(fn `UserConstructionScript`)