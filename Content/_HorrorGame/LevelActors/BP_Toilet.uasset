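; BP_Toilet is an interactable toilet level actor that advances a scripted story task in the horror game.
; An ACTCHighligther component targets the static mesh at BeginPlay and toggles its highlight as anything enters or leaves the Box trigger.
; Interact reports the task about returning to find the planchet moving on its own as completed to the GameMode's ACTCDialogueManager, then prints a debug string.
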(event `self.ReceiveBeginPlay`
  (`/Game/_HorrorGame/Core/ActorComponents/ACTC_Highligther.SetHighlightedActor` (`self.ACTC_Highligther`) (`self.StaticMeshComponent`)))

(event `/Game/_HorrorGame/Core/Interfaces/BPI_Interactable.Interact`
  (bind _asbp_game_mode (cast `/Game/_HorrorGame/Core/GameModes/Gameplay/BP_GameMode` (`GameplayStatics.GetGameMode`)))
  (`/Game/_HorrorGame/Core/DialogueSystem/ACTC_DialogueManager.CompletedTask` (`/Game/_HorrorGame/Core/GameModes/Gameplay/BP_GameMode.ACTC_DialogueManager` _asbp_game_mode) "Returns and surprised that the planchet is moving on its own")
  (`KismetSystemLibrary.PrintString` "interact tiolet"))

(event `self.Box.OnComponentBeginOverlap`
  (params (OverlappedComponent :type "PrimitiveComponent Object Reference") (OtherActor :type "Actor Object Reference") (OtherComp :type "PrimitiveComponent Object Reference") (OtherBodyIndex :type Integer) (bFromSweep :type Boolean) (SweepResult :type "HitResult Structure (by ref)"))
  (`/Game/_HorrorGame/Core/ActorComponents/ACTC_Highligther.HighlightActor` (`self.ACTC_Highligther`) true))

(event `self.Box.OnComponentEndOverlap`
  (params (OverlappedComponent :type "PrimitiveComponent Object Reference") (OtherActor :type "Actor Object Reference") (OtherComp :type "PrimitiveComponent Object Reference") (OtherBodyIndex :type Integer))
  (`/Game/_HorrorGame/Core/ActorComponents/ACTC_Highligther.HighlightActor` (`self.ACTC_Highligther`) false))

(fn `UserConstructionScript`)