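; BP_EnemyBase is an enemy base Blueprint for the horror game, with player-overlap feedback and teleporting toward the player.
; Its Sphere spawns a scaled-up spark effect at the enemy when BP_FirstPersonCharacter overlaps it.
; TeleportAtPlayer delegates to ChaseComponent.
; A looping timer fires an empty ScreamEvent, and the interpolated rotation toward the player is disconnected, so it never runs.
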(event `self.ReceiveBeginPlay`
  (`KismetSystemLibrary.K2_SetTimerDelegate` (delegate `ScreamEvent`) 2.0 true))

(event `ScreamEvent`)

(event `self.Sphere.OnComponentBeginOverlap`
  (params (OverlappedComponent :type "PrimitiveComponent Object Reference") (OtherActor :type "Actor Object Reference") (OtherComp :type "PrimitiveComponent Object Reference") (OtherBodyIndex :type Integer) (bFromSweep :type Boolean) (SweepResult :type "HitResult Structure (by ref)"))
  (cast `/Game/FirstPerson/Blueprints/BP_FirstPersonCharacter` OtherActor)
  (`GameplayStatics.SpawnEmitterAtLocation` "/Game/StarterContent/Particles/P_Sparks.P_Sparks" (`self.K2_GetActorLocation`) (struct) (5.0 5.0 5.0)))

(event `TeleportAtPlayer`
  (`/Game/_HorrorGame/Core/AISystem/AI/ActorComponents/ChaseComponent.TeleportToPlayer` (`self.ChaseComponent`)))

(fn `UserConstructionScript`)