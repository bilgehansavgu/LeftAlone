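; BP_Enemy_Witch is a witch enemy Blueprint in the horror game's AI system that adds a vertical bobbing motion to the actor.
; Tick accumulates time and feeds a sine wave into a swept Z world offset, applied per frame without delta-time scaling, so bob height depends on frame rate.
; The graph holds no other active logic, and the construction script only calls its parent.
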(event `self.ReceiveTick`
  (params (DeltaSeconds :type "Float (single-precision)"))
  (bind _output_get (set `self.T` (+ DeltaSeconds (`self.T`))))
  (`self.K2_AddActorWorldOffset` (`KismetMathLibrary.MakeVector` 0.0 0.0 (* (`KismetMathLibrary.Sin` (* _output_get 2.0)) 10.0)) true))

(fn `UserConstructionScript`
  (`parent.UserConstructionScript`))