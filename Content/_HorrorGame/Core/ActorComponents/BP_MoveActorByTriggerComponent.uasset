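; BP_MoveActorByTriggerComponent is an actor component that teleports its owner once, when a chosen dialogue completes.
; One tick after BeginPlay, it subscribes to the completion event of the dialogue manager on BP_GameMode.
; When the completed key matches DialogueSelectedToMove, it prints the key and offsets the owner's location using random MoveLocations entries.
; A similar dialogue-play handler exists, but its Triggerer binding never runs.
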(event `self.ReceiveBeginPlay`
  (`KismetSystemLibrary.DelayUntilNextTick`)
  (bind _asbp_game_mode (cast `/Game/_HorrorGame/Core/GameModes/Gameplay/BP_GameMode` (`GameplayStatics.GetGameMode`)))
  (add `/Game/_HorrorGame/Core/DialogueSystem/ACTC_DialogueManager.OnCompleteDialogue` (`/Game/_HorrorGame/Core/GameModes/Gameplay/BP_GameMode.ACTC_DialogueManager` _asbp_game_mode) (delegate `OnCompleteDialogue_Event`)))

(event `OnCompleteDialogue_Event`
  (params (`Dialogue Key` :type String))
  (bind _returnvalue (`self.GetOwner`))
  (bind _dialogueselectedtomove (`self.DialogueSelectedToMove`))
  (bind (_returnvalue_x _returnvalue_y _returnvalue_z) (`KismetMathLibrary.BreakVector` (+ (`Actor.K2_GetActorLocation` _returnvalue) (`KismetArrayLibrary.Array_Random` (`self.MoveLocations`)))))
  (if (`KismetStringLibrary.EqualEqual_StrStr` `Dialogue Key` _dialogueselectedtomove)
    (`KismetSystemLibrary.PrintString` _dialogueselectedtomove true true (struct :`R` 0.987481 :`G` 1.0 :`A` 1.0))
    (`/Engine/EditorBlueprintResources/StandardMacros.DoOnce` false
      (:`Completed`
        (`Actor.K2_SetActorLocation` _returnvalue (`KismetMathLibrary.MakeVector` _returnvalue_x _returnvalue_y _returnvalue_z) false true)))))

(event `OnDialoguePlay_Event`
  (params (`Dialogue key` :type String) (`Actor to Focus` :type "Actor Object Reference"))
  (bind _returnvalue (`self.GetOwner`))
  (bind (_returnvalue_x _returnvalue_y _returnvalue_z) (`KismetMathLibrary.BreakVector` (+ (`Actor.K2_GetActorLocation` _returnvalue) (`KismetArrayLibrary.Array_Random` (`self.MoveLocations`)))))
  (`/Engine/EditorBlueprintResources/StandardMacros.DoOnce` false
    (:`Completed`
      (`Actor.K2_SetActorLocation` _returnvalue (`KismetMathLibrary.MakeVector` _returnvalue_x _returnvalue_y _returnvalue_z) false true))))