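; Trigger zone that starts a keyed dialogue when the player character enters its sphere.
; On BeginPlay it registers as a triggerer with the game mode's dialogue manager component.
; Overlap broadcasts the dialogue key and focus actor, then reports the allowed task completed to that manager.
; A self-repeating KeepTalking event can step script lines through a dialogue widget on a delay, but the overlap path does not call it.
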(event `self.ReceiveBeginPlay`
  (bind _returnvalue (`GameplayStatics.GetGameMode`))
  ;[0 0 0 1 30] Beginplay
  (`/Engine/EditorBlueprintResources/StandardMacros.IsValid` _returnvalue
    (:`Is Valid`
      (`/Game/_HorrorGame/Core/DialogueSystem/ACTC_DialogueManager.AddTriggerer` (`self.GetComponentByClass` _returnvalue "/Game/_HorrorGame/Core/DialogueSystem/ACTC_DialogueManager.ACTC_DialogueManager_C") self)
      (bind _asbp_game_mode (cast `/Game/_HorrorGame/Core/GameModes/Gameplay/BP_GameMode` (`GameplayStatics.GetGameMode`)))
      (set `self.Ref BP Game Mode` _asbp_game_mode))))

(event `KeepTalking`
  (if (< (`self.Script Index`) (`KismetArrayLibrary.Array_Length` (`self.DialogueScript`)))
    ;[1 1 1] bad cast
    (cast `/Game/_HorrorGame/Core/Characters/BP_Character` (stale `self.Sphere.OnComponentBeginOverlap` OtherActor))
    (`self.Dialogue Widget`
      (:`then`
        _)
      (:`else`
        (bind _returnvalue (`|CreateWidget` "/Game/_HorrorGame/Core/Widgets/WBP_Dialogue.WBP_Dialogue_C" (`GameplayStatics.GetPlayerController` 0)))
        (bind _output_get (set `self.Dialogue Widget` _returnvalue))
        (`UserWidget.AddToViewport` _output_get 0)))
    (`TextBlock.SetText` (`/Game/_HorrorGame/Core/Widgets/WBP_Dialogue.dialoguetext` (`self.Dialogue Widget`)) (`KismetTextLibrary.Conv_StringToText` (`|GetArrayItem` (`self.DialogueScript`) (`self.Script Index`))))
    (`/Engine/EditorBlueprintResources/StandardMacros.IncrementInt` (`self.Script Index`)
      (:`  `
        (`KismetSystemLibrary.Delay` (`self.Text Delay Time`))
        (`self.KeepTalking`)))
    (else
      (bind _dialogue_widget (`self.Dialogue Widget`)
        (:`then`
          (`Widget.RemoveFromParent` _dialogue_widget))
        (:`else`)))))

(event `self.Sphere.OnComponentBeginOverlap`
  (params (OverlappedComponent :type "PrimitiveComponent Object Reference") (OtherActor :type "Actor Object Reference") (OtherComp :type "PrimitiveComponent Object Reference") (OtherBodyIndex :type Integer) (bFromSweep :type Boolean) (SweepResult :type "HitResult Structure (by ref)"))
  (cast `/Game/_HorrorGame/Core/Characters/BP_Character` OtherActor)
  ;[1 1 1] the dialogue name key given passed in will be allowed to use now, if dialogue is not passed in it cant be used
  (`self.OnDialoguePlay` (`self.DialogueKey`) (`self.Actor To Focus`))
  (`/Game/_HorrorGame/Core/DialogueSystem/ACTC_DialogueManager.CompletedTask` (`/Game/_HorrorGame/Core/GameModes/Gameplay/BP_GameMode.ACTC_DialogueManager` (`self.Ref BP Game Mode`)) (`self.Dialogue Task Allowed`)))

(fn `UserConstructionScript`)