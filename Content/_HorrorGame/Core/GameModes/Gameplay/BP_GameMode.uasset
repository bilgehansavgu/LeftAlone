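; Game mode for the horror game that seeds the story dialogue, from Marty's parents leaving through his Ouija board scare.
; On BeginPlay it completes the opening-dialogue task on ACTCDialogueManager, then binds a handler to that manager's completed-registered-triggers callback.
; The handler adds hardcoded scripts keyed by story beat, each flagged as not yet played.
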(event `self.ReceiveBeginPlay`
  (`|ExecutionSequence`
    (:`then_0`
      ;[1 1 1] init triggerer, marty, Opening dialogue with parents
      (`/Game/_HorrorGame/Core/DialogueSystem/ACTC_DialogueManager.CompletedTask` (`self.ACTC_DialogueManager`) "Opening dialogue with parents"))
    (:`then_1`
      ;[1 1 1] dialogue stuff
      (add `/Game/_HorrorGame/Core/DialogueSystem/ACTC_DialogueManager.OnCompletedRegisteredTriggers` (`self.ACTC_DialogueManager`) (delegate `OnCompletedRegisteredTriggers_Event`)))))

(event `OnCompletedRegisteredTriggers_Event`
  ;[1 1 1] dialogue stuff
  (`/Game/_HorrorGame/Core/DialogueSystem/ACTC_DialogueManager.AddDialogue` (`self.ACTC_DialogueManager`) "Opening dialogue with parents" (make `/Game/_HorrorGame/Core/DialogueSystem/S_Script` (`|MakeArray` "Marty: All right, take care, you guys!" "Dad: We’ll be back late at night. Don’t wait for us, go to bed in time!" "Mom: All right Muffin, there’s fresh pizza on the kitchen counter," "Marty: Okay" "Mom: and drinks in the fridge," "Marty: Okay" "Mom: if anything happens, call us immediately," "Marty: Mom" "Mom: emergency numbers on the fridge door. We’ll hurry home." "Dad: No we won’t." "Marty: Moooom, I’ll be fine." "Dad: Have fun, you’ll be the Lord of the Kingdom tonight Sir Mart." "Marty: I will Sir Ken! You guys have fun too." :!type "Text")))
  (`/Game/_HorrorGame/Core/DialogueSystem/ACTC_DialogueManager.AddDialogue` (`self.ACTC_DialogueManager`) "Let’s do something fun" (make `/Game/_HorrorGame/Core/DialogueSystem/S_Script` (`|MakeArray` "Ooookay, finally the place’s all mine and I’ve got the best things planned out for tonight. First things first, I’m starving." :!type "Text")))
  (`/Game/_HorrorGame/Core/DialogueSystem/ACTC_DialogueManager.AddDialogue` (`self.ACTC_DialogueManager`) "Sitting on the couch" (make `/Game/_HorrorGame/Core/DialogueSystem/S_Script` (`|MakeArray` "Marty: Dude, I’m gonna bust!!! this pizza was awesome! \nAight, enough movies… let’s do something else. I should get it out of my backpack." :!type "Text")))
  (`/Game/_HorrorGame/Core/DialogueSystem/ACTC_DialogueManager.AddDialogue` (`self.ACTC_DialogueManager`) "Getting the Ouija out and start playing" (make `/Game/_HorrorGame/Core/DialogueSystem/S_Script` (`|MakeArray` "Marty: I can’t believe I’m about to try this stupid thing." "Marty: Is someone here? \nMarty (in a separate text bubble): Give me a sign! \nMarty (in a separate text bubble): Can you move the planchet to yes?" "Marty (in a separate text bubble): Is there anyone who would like to speak to me? \nMarty (in a separate text bubble): Is this thing even on? \n" "Marty: Of course, nothing happens." "Marty: This is just a stupid game for babies." "Marty (in a separate text bubble): If YoU dOn’T sEnD mY mEsSaGe To AlL yOuR gHoSt FrIeNdS iN tHe NeXt TwO mInUtEs, YoU wIlL Be CURSED FoReVeR!" "Marty (in a separate text bubble): You hear me ghosts? " "Marty: Yeah, I thought  so… Back to the backpack with you, Scammer Board! Nah.. I’ll deal with you later, I need to go to the toilet." :!type "Text")))
  (`/Game/_HorrorGame/Core/DialogueSystem/ACTC_DialogueManager.AddDialogue` (`self.ACTC_DialogueManager`) "Returns and surprised that the planchet is moving on its own" (make `/Game/_HorrorGame/Core/DialogueSystem/S_Script` (`|MakeArray` "Marty: Okay, I had enough for today. Where’s that stupid boaaaaa……… Is… Is that thing moving on its own? IT IS! WHAT THE FUCK!" "R-U-N" :!type "Text"))))

(fn `UserConstructionScript`)