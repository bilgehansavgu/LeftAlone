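; BP_BaseGrabbable is a base actor for objects held in front of a camera through a physics handle.
; SetupObject stores the handle and camera, and OnObjectGrab returns the static mesh.
; While tick is enabled via EnabledTick, it moves the handle's target to a fixed distance along the camera's forward vector.
; Tick also prints a debug string every frame.
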(event `self.ReceiveTick`
  (params (DeltaSeconds :type "Float (single-precision)"))
  (`KismetSystemLibrary.PrintString` "OBJECTGRABBER")
  (bind _camera (`self.Camera`)
    (:`then`
      (bind _physic_handle (`self.Physic Handle`)
        (:`then`
          (`PhysicsHandleComponent.SetTargetLocation` _physic_handle (+ (`SceneComponent.K2_GetComponentLocation` _camera) (* 100.0 (`SceneComponent.GetForwardVector` _camera)))))
        (:`else`)))
    (:`else`)))

(event `/Game/_HorrorGame/Core/Interfaces/BPI_Grabbable.SetupObject`
  (params (PhysicHandle :type "PhysicsHandleComponent Object Reference") (Camera :type "CameraComponent Object Reference"))
  (set `self.Physic Handle` PhysicHandle)
  (set `self.Camera` Camera))

(event `/Game/_HorrorGame/Core/Interfaces/BPI_Grabbable.EnabledTick`
  (params (Enabled :type Boolean))
  (`self.SetActorTickEnabled` Enabled))

(fn `OnObjectGrab`
  (returns (GrabbedItem :type "PrimitiveComponent Object Reference"))
  (return (`self.StaticMesh`)))

(fn `UserConstructionScript`)